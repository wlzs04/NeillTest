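; GameManager holds the player's PlayerInfo object and grants a door-themed achievement.
; Its Init event constructs PlayerInfo with itself as outer and stores the reference.
; AddTempBool1 uses a flag on PlayerInfo as a one-time guard, then shows a TipUI widget with a Chinese congratulation for "Doors can't stop me!".
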(event EventInit
  (bind _returnvalue (Game|ConstructObjectfromClass "/Game/MyContent/Blueprint/PlayerInfo.PlayerInfo_C" self))
  (Variables|Default|SetPlayerInfo _returnvalue))

(fn AddTempBool1
  (bind _playerinfo (Variables|Default|GetPlayerInfo))
  (if (not (Variables|/Game/MyContent/Blueprint/PlayerInfo.PlayerInfo_C|GettempBool1 _playerinfo))
    (Variables|/Game/MyContent/Blueprint/PlayerInfo.PlayerInfo_C|SettempBool1 _playerinfo true)
    (bind _returnvalue (UserInterface|CreateWidget "/Game/MyContent/UMG/TipUI.TipUI_C" (Game|GetPlayerController 0)))
    (UserInterface|Viewport|AddtoViewport _returnvalue 0)
    (Default|SetText _returnvalue "恭喜完成成就:门拦不住我!")))