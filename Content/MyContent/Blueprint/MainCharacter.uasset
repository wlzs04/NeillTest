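; MainCharacter is the player character Blueprint, handling movement, camera look, jumping and held-button ranged attacks.
; Movement follows control-rotation yaw, and the CanOperate flag gates movement, look and jump input, but not attacking.
; On BeginPlay it spawns a RemoteAttackHelper actor that owns the attack logic and has its focus direction reset by look input.
; RemoteAttack calls the helper immediately, then repeats on a looping timer until released.
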(event Custom|OnFireEvent
  (CallFunction|OnRemoteAttack))

(event EventBeginPlay
  (CallFunction|InitRemoteAttackHelper))

(event Collision|EventActorBeginOverlap
  (params (OtherActor :type Actor%20Object%20Reference)))

(event EventTick
  (params (DeltaSeconds :type Float%20%28single-precision%29)))

(event Input|ActionEvents|InputActionJump
  (params (Key :type Key%20Structure))
  (:Pressed
    (if (Variables|Default|GetcanOperate)
      (Character|Jump))))

(event Input|ActionEvents|InputActionRemoteAttack
  (params (Key :type Key%20Structure))
  (:Pressed
    (Variables|Default|SetinFire true)
    (CallFunction|OnRemoteAttack)
    (bind _returnvalue (Utilities|Time|SetTimerbyEvent (delegate Custom|OnFireEvent) 0.2 true))
    (Variables|Default|SetfireHandler _returnvalue))
  (:Released
    (Variables|Default|SetinFire false)
    (Utilities|Time|ClearandInvalidateTimerbyHandle (Variables|Default|GetfireHandler))))

(event Input|ActionEvents|InputActionRemotePowerAttack
  (params (Key :type Key%20Structure)))

(event Input|AxisEvents|InputAxisMoveForward
  (params (AxisValue :type Float%20%28single-precision%29))
  (if (Variables|Default|GetcanOperate)
    (Pawn|Input|AddMovementInput (.X (Math|Rotator|GetAxes (Math|Rotator|MakeRotator 0.0 0.0 (.Yaw (Math|Rotator|BreakRotator (Pawn|GetControlRotation :!class /Script/Engine.Pawn)))))) AxisValue false)))

(event Input|AxisEvents|InputAxisMoveRight
  (params (AxisValue :type Float%20%28single-precision%29))
  (if (Variables|Default|GetcanOperate)
    (Pawn|Input|AddMovementInput (.Y (Math|Rotator|GetAxes (Math|Rotator|MakeRotator 0.0 0.0 (.Yaw (Math|Rotator|BreakRotator (Pawn|GetControlRotation :!class /Script/Engine.Pawn)))))) AxisValue false)))

(event Input|AxisEvents|InputAxisLookUp
  (params (AxisValue :type Float%20%28single-precision%29))
  (if (Variables|Default|GetcanOperate)
    (Pawn|Input|AddControllerPitchInput (* (* (* AxisValue -1.0) (Variables|Default|GetbaseLookRate)) (Utilities|Time|GetWorldDeltaSeconds)))
    (Default|ResetFocusDirection (Variables|Default|GetremoteAttackHelper))))

(event Input|AxisEvents|InputAxisTurn
  (params (AxisValue :type Float%20%28single-precision%29))
  (if (Variables|Default|GetcanOperate)
    (Pawn|Input|AddControllerYawInput (* (* AxisValue (Variables|Default|GetbaseTurnRate)) (Utilities|Time|GetWorldDeltaSeconds)))
    (Default|ResetFocusDirection (Variables|Default|GetremoteAttackHelper))))

(fn ConstructionScript)

(fn SetCanOperate
  (params (enabled :type Boolean))
  (Variables|Default|SetcanOperate enabled))

(fn InitRemoteAttackHelper
  (bind _returnvalue (Transformation|GetActorTransform))
  (bind _self self)
  (bind (_location _rotation) (Math|Transform|BreakTransform _returnvalue))
  (bind _returnvalue_2 (Game|SpawnActorfromClass "/Game/MyContent/Blueprint/RemoteAttackHelper.RemoteAttackHelper_C" (Math|Transform|MakeTransform _location _rotation) "AlwaysSpawn" _self _self))
  (bind _output_get (Variables|Default|SetremoteAttackHelper _returnvalue_2))
  (Default|SetMainCharacter _output_get self))

(fn OnRemoteAttack
  (bind _remoteattackhelper (Variables|Default|GetremoteAttackHelper))
  (Utilities|IsValid _remoteattackhelper
    (:Is%20Valid
      (Default|Attack _remoteattackhelper))
    (:Is%20Not%20Valid
      (Development|PrintString "远程攻击助手不存在，需要重新生成。"))))