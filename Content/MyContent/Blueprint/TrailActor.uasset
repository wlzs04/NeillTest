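; TrailActor is a short-lived afterimage that shows a frozen copy of a skeletal mesh pose and fades it out.
; ShowPoseByMainCharacter copies the pose from the supplied skeletal component onto a PoseableMesh.
; BeginPlay puts dynamic trail material instances on the first two slots, then destroys the actor after one second.
; Tick lowers Alpha at a matching rate and writes it to each dynamic material for the fade.
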(event EventBeginPlay
  (bind _poseablemesh (Variables|Default|GetPoseableMesh))
  (Rendering|Material|CreateDynamicMaterialInstance _poseablemesh 0 "/Game/MyContent/Material/TrialMaterial_Inst.TrialMaterial_Inst" "None" :!class /Script/Engine.PrimitiveComponent)
  (Rendering|Material|CreateDynamicMaterialInstance _poseablemesh 1 "/Game/MyContent/Material/TrialMaterial_Inst.TrialMaterial_Inst" "None" :!class /Script/Engine.PrimitiveComponent)
  (Utilities|FlowControl|Delay 1.0)
  (Actor|DestroyActor))

(event Collision|EventActorBeginOverlap
  (params (OtherActor :type Actor%20Object%20Reference)))

(event EventTick
  (params (DeltaSeconds :type Float%20%28single-precision%29))
  (bind _poseablemesh (Variables|Default|GetPoseableMesh))
  (bind _output_get (Variables|Default|Setalpha (- (Variables|Default|Getalpha) (* DeltaSeconds 1.0))))
  (for _index (range 0 (Rendering|Material|GetNumMaterials _poseablemesh))
    (bind _asmaterial_instance_dynamic (Utilities|Casting|CastToMaterialInstanceDynamic (Rendering|Material|GetMaterial _poseablemesh _index)))
    (Rendering|Material|SetScalarParameterValue _asmaterial_instance_dynamic "Alpha" _output_get :!class /Script/Engine.MaterialInstanceDynamic)))

(fn ConstructionScript)

(fn ShowPosebyMainCharacter
  (params (NewParam :type Skeletal%20Mesh%20Component%20Object%20Reference))
  (Class|PoseableMeshComponent|CopyPosefromSkeletalComponent (Variables|Default|GetPoseableMesh) NewParam))