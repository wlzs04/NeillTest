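; RemoteAttackHelper is a companion actor that follows the main character and fires projectiles.
; MoveToMainCharacter targets the nearer of two raised points beside the character, stopping when close and teleporting when too far.
; Tick sweeps toward that target at constant speed, refreshing it every frame while moving and on a timed interval while idle.
; Attack launches a BulletBase with force along the mesh's facing, which ResetFocusDirection sets from player control rotation.
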(event EventBeginPlay)

(event Collision|EventActorBeginOverlap
  (params (OtherActor :type Actor%20Object%20Reference)))

(event EventTick
  (params (DeltaSeconds :type Float%20%28single-precision%29))
  (bind _returnvalue (Actor|GetGameTimeSinceCreation))
  (if (Variables|Default|GetneedMove)
    (Utilities|FlowControl|Sequence
      (:then_0
        ;[1 1 1] 判断助手是否需要移动
        (CallFunction|MovetoMainCharacter :!label _label)
        (Variables|Default|SetlastTime _returnvalue))
      (:then_1
        (Transformation|AddActorLocalOffset self (* (Math|Vector|Normalize (- (Variables|Default|GetneedMoveLocation) (Transformation|GetActorLocation))) (* (Variables|Default|Getspeed) DeltaSeconds)) true false)))
    (elif (>= (- _returnvalue (Variables|Default|GetlastTime)) (Variables|Default|GetresetTrasformTimeDetal))
      (goto _label))))

(fn ConstructionScript)

(fn SetMainCharacter
  (params (mainCharacter :type Main%20Character%20Object%20Reference))
  (Variables|Default|SetmyMainCharacter mainCharacter))

(fn MovetoMainCharacter
  (bind _returnvalue (Transformation|GetActorLocation))
  (bind _mymaincharacter (Variables|Default|GetmyMainCharacter))
  (bind _returnvalue_2 (Transformation|GetActorRotation _mymaincharacter))
  (bind _returnvalue_3 (Transformation|GetActorLocation _mymaincharacter))
  (bind _returnvalue_4 (Math|Vector|GetRightVector _returnvalue_2))
  (bind _returnvalue_5 (+ _returnvalue_3 "0, 0,50.000000"))
  (bind _returnvalue_6 (* _returnvalue_4 5e+01))
  (bind _returnvalue_7 (- "0, 0, 0" _returnvalue_6))
  (bind _returnvalue_8 (+ _returnvalue_5 _returnvalue_6))
  (bind _returnvalue_9 (- _returnvalue _returnvalue_8))
  (bind _returnvalue_10 (+ _returnvalue_5 _returnvalue_7))
  (bind _returnvalue_11 (Math|Vector|VectorLength _returnvalue_9))
  (bind _returnvalue_12 (- _returnvalue _returnvalue_10))
  (bind _returnvalue_13 (Math|Vector|VectorLength _returnvalue_12))
  ;[1 1 1] 获得两个Actor之间的距离
  (if (< _returnvalue_11 _returnvalue_13)
    (LocalVariables|SethelperLoaction _returnvalue_8)
    (LocalVariables|SetlocationLength _returnvalue_11)
    (else
      (LocalVariables|SethelperLoaction _returnvalue_10)
      (LocalVariables|SetlocationLength _returnvalue_13)))
  ;[1 1 1] 当距离小于规定移动的最小距离时
  (if (< (LocalVariables|GetlocationLength) (Variables|Default|GetminMoveLength))
    (Variables|Default|SetneedMove false)
    (else
      ;[1 1 1] 当距离超过规定移动的最大距离时
      (if (> (LocalVariables|GetlocationLength) (Variables|Default|GetmaxMoveLength))
        ;[1 1 1] 移动助手到指定位置
        (Transformation|AddActorLocalOffset (- (LocalVariables|GethelperLoaction) (Transformation|GetActorLocation)) false true)
        (else
          ;[1 1 1] 添加移动组手动画
          (Variables|Default|SetneedMove true)
          (Variables|Default|SetneedMoveLocation (LocalVariables|GethelperLoaction)))))))

(fn Attack
  (bind _staticmesh (Variables|Default|GetStaticMesh))
  (bind _returnvalue (Transformation|GetWorldTransform _staticmesh))
  (bind (_location _rotation) (Math|Transform|BreakTransform _returnvalue))
  (bind _returnvalue_2 (Game|SpawnActorfromClass "/Game/MyContent/Blueprint/BulletBase.BulletBase_C" (Math|Transform|MakeTransform _location _rotation) "AlwaysSpawn" self 0))
  (Physics|AddForce (Variables|/Game/MyContent/Blueprint/BulletBase.BulletBase_C|GetStaticMesh _returnvalue_2) (* (Math|Rotator|GetRotationXVector (Variables|/Script/Engine.SceneComponent|GetRelativeRotation (Variables|Default|GetStaticMesh))) 3e+03) "None" false))

(fn ResetFocusDirection
  (Transformation|SetRelativeRotation (Variables|Default|GetStaticMesh) (Pawn|GetControlRotation (Game|GetPlayerController 0) :!class /Script/Engine.Controller) false false))