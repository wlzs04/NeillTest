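; Player controller that toggles a debug overlay and can show a welcome screen.
; It creates the DebugUI widget once on BeginPlay, then key 1 adds or removes it from the viewport.
; While the overlay is open, the mouse cursor is visible and input on player character 0 is disabled.
; A separate ShowWelcomeUI function creates and displays a WelcomeUI widget, with no caller in this graph.
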(event EventBeginPlay
  (bind _returnvalue (UserInterface|CreateWidget "/Game/MyContent/UMG/DebugUI.DebugUI_C"))
  (Variables|Default|SetDebugUI _returnvalue))

(event EventTick
  (params (DeltaSeconds :type Float%20%28single-precision%29)))

(event Input|KeyboardEvents|1
  (params (Key :type Key%20Structure))
  (bind _self self)
  (:Pressed
    (if (Variables|Default|GetdebugShowing)
      (Widget|RemovefromParent (Variables|Default|GetdebugUI))
      (Variables|Default|SetdebugShowing false)
      (Variables|Default|SetbShowMouseCursor false)
      (Input|EnableInput (Game|GetPlayerCharacter 0) _self)
      (else
        (UserInterface|Viewport|AddtoViewport (Variables|Default|GetdebugUI) 0)
        (Variables|Default|SetdebugShowing true)
        (Variables|Default|SetbShowMouseCursor true)
        (Input|DisableInput (Game|GetPlayerCharacter 0) _self)))))

(fn ConstructionScript)

(fn ShowWelcomeUI
  (bind _returnvalue (UserInterface|CreateWidget "/Game/MyContent/UMG/WelcomeUI.WelcomeUI_C"))
  (UserInterface|Viewport|AddtoViewport _returnvalue 0))